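; Boss enemy character with melee and jump attacks, whose death triggers the win screen.
; Pawn sensing writes the seen player to the AI blackboard, clearing it if that player is dead.
; Attack events hold RepNotify flags for three seconds; the jump attack then launches along a suggested arc toward its target.
; Tick updates the overhead health bar and, once at zero health, stops movement, disables collision and shows the win widget on non-authority clients.
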(event OnSeePawn(PawnSensingComponent)
  (params (Pawn :type Pawn%20Object%20Reference))
  (bind _asbp_top_down_character (Utilities|Casting|CastToBP_TopDownCharacter Pawn))
  (AI|Components|Blackboard|SetValueasBool (CallFunction|TargetBlackBoard) (Utilities|Name|MakeLiteralName "hasSeenPlayer") true)
  (if (<= (Variables|/Script/BanSungOnline.BanSungOnlineCharacter|GetHealth _asbp_top_down_character) 0.0)
    (AI|Components|Blackboard|SetValueasBool (CallFunction|TargetBlackBoard) (Utilities|Name|MakeLiteralName "hasSeenPlayer") false)
    (AI|Components|Blackboard|SetValueasObject (CallFunction|TargetBlackBoard) (Utilities|Name|MakeLiteralName "TargetPlayer") 0)
    (else
      (AI|Components|Blackboard|SetValueasObject (CallFunction|TargetBlackBoard) (Utilities|Name|MakeLiteralName "TargetPlayer") _asbp_top_down_character))))

(event Custom|Attack
  (Variables|Default|SetAttack%20melee true)
  (Utilities|FlowControl|Delay 3.0)
  (Variables|Default|SetAttack%20melee false))

(event Custom|JumpAttack
  (params (Attack%20Target :type Vector))
  (Variables|Default|SetAttack%20range true)
  (Utilities|FlowControl|Delay 3.0)
  (Variables|Default|SetAttack%20range false)
  (bind _outlaunchvelocity (Game|SuggestProjectileVelocityCustomArc (Transformation|GetActorLocation) (Math|Vector|MakeVector (- (.x Attack%20Target) 2.0) (.y Attack%20Target) (+ (.z Attack%20Target) 1e+02)) 1.0 0.5))
  (Character|LaunchCharacter _outlaunchvelocity true true))

(event EventTick
  (params (DeltaSeconds :type Float%20%28single-precision%29))
  (Utilities|FlowControl|Sequence
    (:then_0
      (if (<= (Variables|Default|GetHealth) 0.0)
        (Utilities|FlowControl|DoOnce false
          (:Completed
            (Components|Movement|StopMovementImmediately (Variables|Character|GetCharacterMovement))
            (Development|SetHiddeninGame (Variables|Default|GetWidget%20Component) true false)
            (Collision|SetCollisionEnabled (Variables|Default|GetCapsuleComponent) "NoCollision")
            (Networking|SwitchHasAuthority
              (:Remote
                (bind _returnvalue (UserInterface|CreateWidget "/Game/UI/WBP_WinGame.WBP_WinGame_C"))
                (UserInterface|Viewport|AddtoViewport _returnvalue 0)))))))
    (:then_1
      (bind _aswbp_health_enemy (Utilities|Casting|CastToWBP_HealthEnemy (UserInterface|GetWidget (Variables|Default|GetWidget%20Component))))
      (Progress|SetPercent (Variables|/Game/UI/WBP_HealthEnemy.WBP_HealthEnemy_C|GetHealrh_bar _aswbp_health_enemy) (/ (Variables|Default|GetHealth) (Variables|Default|GetMaxHealth))))))

(fn ConstructionScript)

(fn OnRepAttackMelee)

(fn OnRepAttackRange)

(fn TargetBlackBoard
  (return (AI|GetBlackboard (AI|GetAIController self))))