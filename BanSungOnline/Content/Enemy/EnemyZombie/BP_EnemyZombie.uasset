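; Zombie enemy character that roams random nearby points and, on sighting a pawn, chases the nearest cached BP_TopDownCharacter.
; A retriggerable three-second delay after each sighting returns it to roaming.
; A looping timer set at BeginPlay fires melee attacks regardless of range, toggling replicated AttackMele only on the Remote authority branch.
; Tick updates the overhead health bar and, at zero health, stops movement, hides the widget and disables capsule collision.
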(event OnSeePawn(PawnSensingComponent)
  (params (Pawn :type Pawn%20Object%20Reference))
  (Variables|Default|Setmin 1e+15)
  (for (_array_element _array_index) (Variables|Default|GetNewVar)
    (if (< (Math|Vector|Distance(Vector) (Transformation|GetActorLocation _array_element) (Transformation|GetActorLocation)) (Variables|Default|Getmin))
      (Variables|Default|Setmin (Math|Vector|Distance(Vector) (Transformation|GetActorLocation _array_element) (Transformation|GetActorLocation)))
      (Variables|Default|SetArray%20Index _array_index)))
  (Utilities|FlowControl|Sequence
    (:then_0
      (AI|AIMoveTo self "0, 0, 0" (Utilities|Array|Get(acopy) (Variables|Default|GetNewVar) (Variables|Default|GetArray%20Index)) 5.0 false))
    (:then_1
      (Utilities|FlowControl|RetriggerableDelay 3.0)
      (CallFunction|Roaming))))

(event Custom|Roaming
  (AI|AIMoveTo self (.RandomLocation (AI|Navigation|GetRandomReachablePointinRadius (Transformation|GetWorldLocation (Variables|Character|GetMesh)) 1e+03 0 0)) 0 5.0 false
    (:OnSuccess
      (Utilities|FlowControl|Delay (Math|Random|RandomFloatinRange 1.0 4.0))
      (CallFunction|Roaming))))

(event Custom|Attack
  (Networking|SwitchHasAuthority
    (:Remote
      (Variables|Default|SetAttackMele true)
      (Utilities|FlowControl|Delay 1.4)
      (Class|Enemy|AttackCharacter)
      (Variables|Default|SetAttackMele false))))

(event Custom|Attackk
  (CallFunction|Attack))

(event EventBeginPlay
  (CallFunction|Roaming)
  (Utilities|FlowControl|Delay 2.0)
  (bind _outactors (Actor|GetAllActorsOfClass "/Game/TopDown/Blueprints/BP_TopDownCharacter.BP_TopDownCharacter_C"))
  (for _array_element _outactors
    (Utilities|Array|Add (Variables|Default|GetNewVar) _array_element)
    (Utilities|Time|SetTimerbyEvent (delegate Custom|Attackk) 2.0 true)))

(event EventTick
  (params (DeltaSeconds :type Float%20%28single-precision%29))
  (bind _charactermovement (Variables|Character|GetCharacterMovement))
  (Utilities|FlowControl|Sequence
    (:then_0
      (if (<= (Variables|Default|GetHealth) 0.0)
        (Components|Movement|StopMovementImmediately _charactermovement)
        (Variables|/Script/Engine.CharacterMovementComponent|SetMaxWalkSpeed _charactermovement 0.0)
        (Development|SetHiddeninGame (Variables|Default|GetWidget%20Component) true false)
        (Collision|SetCollisionEnabled (Variables|Default|GetCapsuleComponent) "NoCollision")))
    (:then_1
      (bind _aswbp_health_enemy (Utilities|Casting|CastToWBP_HealthEnemy (UserInterface|GetWidget (Variables|Default|GetWidget%20Component))))
      (Progress|SetPercent (Variables|/Game/UI/WBP_HealthEnemy.WBP_HealthEnemy_C|GetHealrh_bar _aswbp_health_enemy) (/ (Variables|Default|GetHealth) (Variables|Default|GetMaxHealth))))))

(fn ConstructionScript)

(fn OnRepAttackMele)